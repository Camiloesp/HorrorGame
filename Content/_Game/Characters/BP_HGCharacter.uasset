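; Player character Blueprint that smooths the capsule height change for crouching and shows a flashlight battery debug readout.
; ShortenPlayerCapsule plays a timeline that lerps the capsule half-height from a hardcoded standing value to the movement component's CrouchHalfHeight, updating overlaps.
; LengthenPlayerCapsule reverses the same timeline to restore standing height.
; Tick prints the flashlight component's current battery level every frame for debugging.
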(event EventBeginPlay)

(event Collision|EventActorBeginOverlap
  (params (OtherActor :type Actor%20Object%20Reference)))

(event EventTick
  (params (DeltaSeconds :type Float%20%28single-precision%29))
  ;[1 1 1] Debug
  (Development|PrintString (Utilities|String|ToString(Float) (Variables|/Script/HorrorGame.FlashlightComponent|GetCurrentBatteryLevel (Variables|Default|GetFlashlightComponent))) true true "(R=1.000000,G=0.835470,B=0.000000,A=1.000000)" DeltaSeconds))

(event EventShortenPlayerCapsule
  (bind _alpha (Timeline|Capsule_TL Play)
    (:Update
      (Components|Capsule|SetCapsuleHalfHeight (Variables|Default|GetCapsuleComponent) (Math|Float|Lerp 88.0 (Variables|/Script/HorrorGame.Movement|GetCrouchHalfHeight (Variables|Default|GetHGMovementComp)) _alpha) true))))

(event EventLengthenPlayerCapsule
  (bind _alpha (Timeline|Capsule_TL Reverse)
    (:Update
      (Components|Capsule|SetCapsuleHalfHeight (Variables|Default|GetCapsuleComponent) (Math|Float|Lerp 88.0 (Variables|/Script/HorrorGame.Movement|GetCrouchHalfHeight (Variables|Default|GetHGMovementComp)) _alpha) true))))

(fn ConstructionScript)