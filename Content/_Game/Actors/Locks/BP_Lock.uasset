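; BP_Lock is a combination lock actor that plays its open animation when the dialed code is correct.
; On BeginPlay it enables input from the player controller, and H, J, K and L each rotate one of four dials.
; Every rotation restarts a shared one-second retriggerable delay, so CheckCode runs only once turning pauses.
; Debug prints show the combination every tick and the result of each check.
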(event EventBeginPlay
  (Input|EnableInput (.AsBP%20HGPlayer%20Controller (Utilities|Casting|CastToBP_HGPlayerController (Game|GetPlayerController 0)))))

(event Collision|EventActorBeginOverlap
  (params (OtherActor :type Actor%20Object%20Reference)))

(event EventTick
  (params (DeltaSeconds :type Float%20%28single-precision%29))
  (bind _lockcombination (Variables|Default|GetLockCombination))
  (Development|PrintString (Utilities|String|Append "combination is: " (Utilities|String|ToString(Integer) (Utilities|Array|Get(acopy) _lockcombination)) " " (Utilities|String|ToString(Integer) (Utilities|Array|Get(acopy) _lockcombination 1)) " " (Utilities|String|ToString(Integer) (Utilities|Array|Get(acopy) _lockcombination 2)) " " (Utilities|String|ToString(Integer) (Utilities|Array|Get(acopy) _lockcombination 3))) true true "(R=0.000000,G=0.660000,B=1.000000,A=1.000000)" DeltaSeconds))

(event Input|KeyboardEvents|H
  (params (Key :type Key%20Structure :default "None"))
  (:Pressed
    (Class|LockDial|RotateDial (Utilities|Array|Get(acopy) (Variables|Default|GetDials)))
    (Utilities|FlowControl|RetriggerableDelay 1.0)
    (bind _returnvalue (Class|Lock|CheckCode))
    (Development|PrintString (Utilities|String|ToString(Boolean) _returnvalue))
    (if _returnvalue
      (Components|Animation|PlayAnimation (Variables|Default|GetLockMesh) "/Game/_Game/Props/Lock/LockOpen.LockOpen" false))))

(event Input|KeyboardEvents|J
  (params (Key :type Key%20Structure :default "None"))
  (:Pressed
    (Class|LockDial|RotateDial (Utilities|Array|Get(acopy) (Variables|Default|GetDials) 1))
    (Utilities|FlowControl|RetriggerableDelay 1.0)
    (bind _returnvalue (Class|Lock|CheckCode))
    (Development|PrintString (Utilities|String|ToString(Boolean) _returnvalue))
    (if _returnvalue
      (Components|Animation|PlayAnimation (Variables|Default|GetLockMesh) "/Game/_Game/Props/Lock/LockOpen.LockOpen" false))))

(event Input|KeyboardEvents|K
  (params (Key :type Key%20Structure :default "None"))
  (:Pressed
    (Class|LockDial|RotateDial (Utilities|Array|Get(acopy) (Variables|Default|GetDials) 2))
    (Utilities|FlowControl|RetriggerableDelay 1.0)
    (bind _returnvalue (Class|Lock|CheckCode))
    (Development|PrintString (Utilities|String|ToString(Boolean) _returnvalue))
    (if _returnvalue
      (Components|Animation|PlayAnimation (Variables|Default|GetLockMesh) "/Game/_Game/Props/Lock/LockOpen.LockOpen" false))))

(event Input|KeyboardEvents|L
  (params (Key :type Key%20Structure :default "None"))
  (:Pressed
    (Class|LockDial|RotateDial (Utilities|Array|Get(acopy) (Variables|Default|GetDials) 3))
    (Utilities|FlowControl|RetriggerableDelay 1.0)
    (bind _returnvalue (Class|Lock|CheckCode))
    (Development|PrintString (Utilities|String|ToString(Boolean) _returnvalue))
    (if _returnvalue
      (Components|Animation|PlayAnimation (Variables|Default|GetLockMesh) "/Game/_Game/Props/Lock/LockOpen.LockOpen" false))))

(fn ConstructionScript)